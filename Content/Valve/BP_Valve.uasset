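; BP_Valve is an interactable valve actor that loses health over time.
; Interact toggles a timeline rotating the Cube 90 degrees and flags Finished.
; After a random start delay, BeginPlay repeatedly applies damage with force feedback, camera shake, sound and effects until Finished, then deals one larger delayed hit, resets the flag and stops.
; ApplyDamage prints health and destroys the actor if IsValveDead reports true, though that check's nodes appear unwired.
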(event `/Game/Blueprints/BPI_InteractionInterface.Interact`
  (if (not (`self.IsValveMoving?`))
    (set `self.IsValveMoving?` true)
    (bind _output_get (set `self.Rotating?` (not (`self.Rotating?`))))
    (if _output_get
      (bind (_direction _alpha) (`Timeline|RotateValve` :!label _label)
        (:`Update`
          ; Change return value if the valve asset rotates on a different Roll, Pitch, or yaw
          (`SceneComponent.K2_SetRelativeRotation` (`self.Cube`) (`KismetMathLibrary.MakeRotator` 0.0 (`KismetMathLibrary.Lerp` 0.0 90.0 _alpha)) false false)
          (set `self.Finished?` true))
        (:`Finished`
          (set `self.IsValveMoving?` false)))
      (else
        (goto _label :!via `Reverse`)))))

(event `IncreaseDamgeValve`
  (`self.ApplyDamage` 15))

(event `ValveDeath`
  (`KismetSystemLibrary.PrintString` "The valve has been destroyed."))

(event `self.ReceiveBeginPlay`
  ; To start damaging the valve's health after a 5 second delay, then after the player interacts with the vavle it a short delay before it increases the amount of damage by 5.
  ;; makes the start time of the valves random (hopefully each one is random now)
  (`KismetSystemLibrary.Delay` (`KismetArrayLibrary.Array_Random` (`|MakeArray` 2.5 3.0 3.5 4.0 4.5 5.0 :!type "Float (single-precision)")))
  (`KismetSystemLibrary.Delay` 2.0 :!label _label_2)
  (`GameplayStatics.SpawnForceFeedbackAtLocation` "/Game/ForceFeedback/FFE_ValveOpen.FFE_ValveOpen" (`self.K2_GetActorLocation`) (struct) false 1.0 0.0 "/Game/ForceFeedback/FFA_Default.FFA_Default")
  (`LegacyCameraShake.StartLegacyCameraShakeFromSource` (`GameplayStatics.GetPlayerCameraManager` 0) "/Game/CameraShake/LCS_OpenValve.LCS_OpenValve_C")
  (`GameplayStatics.PlaySoundAtLocation` null (`self.K2_GetActorLocation`) (struct) 1.0 1.0 0.0 null null null null)
  (`NiagaraFunctionLibrary.SpawnSystemAtLocation` null (`self.K2_GetActorLocation`))
  (`self.ApplyDamage` 10)
  (if (`self.Finished?`)
    (`KismetSystemLibrary.Delay` 5.0)
    (`self.IncreaseDamgeValve`)
    ; resets "finished?" value so cycle can restart
    (set `self.Finished?` false)
    (else
      (goto _label_2))))

(fn `ApplyDamage`
  (params (Amount :type Integer))
  (bind _output_get (set `self.VavleHealth` (- (`self.VavleHealth`) Amount)))
  (`KismetSystemLibrary.PrintString` (`KismetTextLibrary.Conv_TextToString` (`|FormatText` "Vavle health {health}" _output_get)))
  (if (`self.IsValveDead?`)
    (`self.ValveDeath`)
    (`self.K2_DestroyActor`)))

(fn `UserConstructionScript`)